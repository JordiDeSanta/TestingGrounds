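; BP_Tile is an endless-terrain tile that chains copies of itself as the third-person character moves through, gated by a lockable wall.
; When the character enters LockingVolume, it spawns the next tile at the Arrow's transform, passing itself as PreviousTile, and unlocks Wall4 (green, no collision).
; Leaving the volume relocks the wall (red, solid) and, after a short delay, destroys the previous tile.
; Spawned tiles start locked.
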(event `self.LockingVolume.OnComponentBeginOverlap`
  (params (OverlappedComponent :type "PrimitiveComponent Object Reference") (OtherActor :type "Actor Object Reference") (OtherComp :type "PrimitiveComponent Object Reference") (OtherBodyIndex :type Integer) (bFromSweep :type Boolean) (SweepResult :type "HitResult Structure (by ref)"))
  (cast `/Game/Dynamic/NPC/Behaviour/BP_TPCharacter` OtherActor)
  (`|SpawnActorFromClass` "BP_Tile_C" (`self.GetAttachLocation`) "Undefined" "OverrideRootScale" null self true null)
  (`self.Unlock`))

(event `self.LockingVolume.OnComponentEndOverlap`
  (params (OverlappedComponent :type "PrimitiveComponent Object Reference") (OtherActor :type "Actor Object Reference") (OtherComp :type "PrimitiveComponent Object Reference") (OtherBodyIndex :type Integer))
  (bind _previoustile (`self.PreviousTile`))
  (cast `/Game/Dynamic/NPC/Behaviour/BP_TPCharacter` OtherActor)
  (`self.Lock`)
  (`KismetSystemLibrary.Delay` 0.2)
  (`/Engine/EditorBlueprintResources/StandardMacros.IsValid` _previoustile
    (:`Is Valid`
      (`self.K2_DestroyActor` _previoustile))))

(event `self.ReceiveBeginPlay`
  (if (`self.Spawned?`)
    (`self.Lock`)))

(fn `GetAttachLocation`
  (returns (AttachTransform :type "Transform Structure"))
  (return (`SceneComponent.K2_GetComponentToWorld` (`self.Arrow`))))

(fn `Lock`
  (bind _wall4 (`self.Wall4`))
  (`PrimitiveComponent.SetMaterial` _wall4 0 "/Game/Static/Materials/MI_Red.MI_Red")
  (`PrimitiveComponent.SetCollisionEnabled` _wall4 "QueryAndPhysics"))

(fn `Unlock`
  (bind _wall4 (`self.Wall4`))
  (`PrimitiveComponent.SetMaterial` _wall4 0 "/Game/Static/Materials/MI_Green.MI_Green")
  (`PrimitiveComponent.SetCollisionEnabled` _wall4 "NoCollision"))

(fn `UserConstructionScript`)